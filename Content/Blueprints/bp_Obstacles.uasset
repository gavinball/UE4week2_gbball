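; bp_Obstacles is an obstacle actor that drifts in a straight line and removes itself after a fixed lifetime.
; The construction script gives it a random yaw, which sets its direction of travel.
; Each Tick accumulates lifespan and offsets the actor along its forward vector by MovementSpeed without sweep or delta-time scaling, then destroys it once it has lived past twenty seconds.
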(event `self.ReceiveBeginPlay`)

(event `self.ReceiveTick`
  (params (DeltaSeconds :type "Float (single-precision)"))
  (bind _output_get (set `self.Lifespan` (+ (`self.Lifespan`) DeltaSeconds)))
  (`/Engine/EditorBlueprintResources/StandardMacros.CompareFloat` _output_get 20.0
    (:`>`
      (`self.K2_DestroyActor`))
    (:`<`
      (`self.K2_AddActorWorldOffset` (* (`KismetMathLibrary.GetForwardVector` (`self.K2_GetActorRotation`)) (`self.Movement Speed`))))))

(fn `UserConstructionScript`
  (`self.K2_SetActorRotation` (`KismetMathLibrary.MakeRotator` 0.0 0.0 (`KismetMathLibrary.RandomFloatInRange` 0.0 360.0))))